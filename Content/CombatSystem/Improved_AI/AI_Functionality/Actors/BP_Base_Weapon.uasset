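; BP_Base_Weapon is a base weapon actor that handles socket attachment and the switch to simulated physics.
; Toggling weapon combat reattaches the actor to its hand socket when enabled and to its attach socket when disabled.
; SimulateWeaponPhysics sets the item mesh to the PhysicsActor collision profile and turns on physics simulation.
; GetCollisionMeshComponent is an empty function, and BeginPlay adds no logic.
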(event Custom|Simulate%20Weapon%20Physics
  (bind _returnvalue (CallFunction|GetItemMesh))
  (Collision|SetCollisionProfileName _returnvalue "PhysicsActor" true :!class /Script/Engine.PrimitiveComponent)
  (Physics|SetSimulatePhysics _returnvalue true))

(event Custom|Toggle%20Weapon%20Combat
  (params (bEnableCombat :type Boolean))
  (CallFunction|AttachActor (select bEnableCombat (Variables|Initialisation|GetHandSocketName) (Variables|Default|GetAttachSocketName))))

(event EventBeginPlay)

(event Collision|EventActorBeginOverlap
  (params (OtherActor :type Actor%20Object%20Reference))
  (|CallParentFunction OtherActor) ; This node is disabled and will not be called.\nDrag off pins to build functionality.
)

(event EventTick
  (params (DeltaSeconds :type Float%20%28single-precision%29))
  (|CallParentFunction DeltaSeconds) ; This node is disabled and will not be called.\nDrag off pins to build functionality.
)

(fn ConstructionScript
  (|CallParentFunction))

(fn GetCollisionMeshComponent)