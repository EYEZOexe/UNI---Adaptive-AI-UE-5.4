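; BP_AI_PatrolRoute is a spline-based patrol path actor that AI characters follow point by point.
; It tracks a current index and direction, exposing that spline point as a world-space location.
; NextPatrolRoute steps the index and flips direction at either end, so patrols ping-pong along the route instead of looping.
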(event Custom|Next%20Patrol%20Route
  (bind _output_get (Variables|Default|SetAI%20Patrol%20Index (+ (Variables|Default|GetAI%20Patrol%20Index) (Variables|Default|GetAI%20Direction))))
  (if (== _output_get (- (Spline|GetNumberOfSplinePoints (Variables|Default|GetAI%20Route)) 1))
    (Variables|Default|SetAI%20Direction -1)
    (elif (== (Variables|Default|GetAI%20Patrol%20Index) 0)
      (Variables|Default|SetAI%20Direction 1))))

(fn ConstructionScript)

(fn GetAISplineRouteasWorldPosition
  (return (Spline|GetLocationatSplinePoint (Variables|Default|GetAI%20Route) (Variables|Default|GetAI%20Patrol%20Index) "World")))