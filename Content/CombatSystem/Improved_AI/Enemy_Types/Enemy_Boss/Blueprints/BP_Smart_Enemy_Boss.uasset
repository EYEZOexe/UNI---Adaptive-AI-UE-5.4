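; Boss enemy character, child of a smart-enemy base, with a boss health bar updated on damage and a spawned, socket-attached weapon.
; Attack events hand melee, jump and ground-smash moves to BACUniversalAttacks, or play montages whose notifies trigger weapon collision, AOE damage, homing weapon throws and lightning strikes.
; A floating-platform phase makes the boss invincible, spawns a platform and signals combat readiness or disengagement when its float timeline ends.
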(event Custom|AI%20Boss%20Attack:%202%20Hit%20Combo
  (params (Attack%20Target :type Actor%20Object%20Reference))
  ;[0.7999 0.8475 1] AI Boss: Attacks
  (Default|ActorMeleeAttack:ShortRange (Variables|Default|GetBAC_Universal_Attacks) (Utilities|Struct|MakeS_AttackInfo Attack%20Target "/Game/Animations/Axe/AM_AI_Boss_2HitCombo.AM_AI_Boss_2HitCombo" (Utilities|Struct|MakeS_DamageInfo 15.0 "NewEnumerator1" "NewEnumerator1" false true true)) 2e+01))

(event Custom|AI%20Boss%20Attacks:%203%20Hit%20Combo%20With%20AOE
  (params (AI%20Attack%20Target :type Actor%20Object%20Reference))
  ;[0.7999 0.8475 1] AI Boss: Attacks
  (CallFunction|AIAttack AI%20Attack%20Target)
  (bind _notifyname (Animation|Montage|PlayMontage (Variables|Character|GetMesh) "/Game/Animations/Axe/AM_AI_Boss_3HitComboWithAOE.AM_AI_Boss_3HitComboWithAOE")
    (:OnCompleted
      (CallFunction|AIEndAttack AI%20Attack%20Target :!label _label))
    (:OnInterrupted
      (goto _label))
    (:OnNotifyBegin
      (switch name _notifyname
        (:Weapon%20Slash
          (Default|ActivateWeaponCollision (Variables|Default|GetBAC_Universal_Attacks) 2e+01 (Utilities|Struct|MakeS_DamageInfo 15.0 "NewEnumerator1" "NewEnumerator1" false true true) "None"))
        (:AOE%20Weapon%20Slash
          (Default|ActorAOEDamage (Variables|Default|GetBAC_Universal_Attacks) 3e+02 (Utilities|Struct|MakeS_DamageInfo 25.0 "NewEnumerator3" "NewEnumerator1" false false false true)))))
    (:OnNotifyEnd
      (switch name _notifyname
        (:Weapon%20Slash
          (Default|DeactivateWeaponCollision (Variables|Default|GetBAC_Universal_Attacks)))))))

(event Custom|On%20Platform%20Float%20Timeline%20End_Event_0
  ;[0.7999 0.8475 1] AI Boss: Floating Platform
  (EventDispatchers|UnbindEventfromOnPlatformFloatTimelineEnd (stale Custom|AI%20Boss%20Attacks:%20Exit%20Floating%20Platform _ai_boss_floating_platform) (delegate Custom|On%20Platform%20Float%20Timeline%20End_Event_0))
  (Actor|DestroyActor (stale Custom|AI%20Boss%20Attacks:%20Exit%20Floating%20Platform _ai_boss_floating_platform))
  (Class|BPICanbeDamaged|IsActorInvinsible(Message) (Variables|Default|GetBAC_DamageSystem) false)
  (Default|CallOnFloatingPlatformCombatDisengage))

(event Custom|AI%20Boss%20Attacks:%20AOE%20Trail
  (params (AI%20Attack%20Target :type Actor%20Object%20Reference))
  ;[0.7999 0.8475 1] AI Boss: Attacks
  (CallFunction|AIAttack AI%20Attack%20Target)
  (bind _notifyname (Animation|Montage|PlayMontage (Variables|Character|GetMesh) "/Game/Animations/Axe/AM_AI_Boss_Ultimate.AM_AI_Boss_Ultimate")
    (:OnCompleted
      (CallFunction|AIEndAttack AI%20Attack%20Target :!label _label))
    (:OnInterrupted
      (goto _label))
    (:OnNotifyBegin
      (switch name _notifyname
        (:Strike
          (bind _returnvalue (Game|SpawnActorfromClass "/Game/CombatSystem/Improved_AI/Improved_DamageSystem/AOE/BP_AOE_LightningStrike.BP_AOE_LightningStrike_C" (Math|Transform|MakeTransform "0, 0, 0" "0, 0, 0" "1.000000,1.000000,1.000000") "Undefined" "MultiplyWithRoot" 0 1.0 AI%20Attack%20Target "/Game/CombatSystem/Improved_AI/Improved_DamageSystem/AOE/Decals/Decal_AOE_LightningStrike.Decal_AOE_LightningStrike" false false false 0))
          (EventDispatchers|AssignOnAOECollisionwithActor _returnvalue (delegate Custom|On%20AOE%20Collision%20With%20Actor_Event)))))))

(event Custom|On%20AOE%20Collision%20With%20Actor_Event
  (params (Actor :type Actor%20Object%20Reference))
  ;[0.7999 0.8475 1] AI Boss: Attacks
  (bind _actor_team_number (Class|BPICanbeDamaged|GetActorTeamNumber(Message) Actor))
  (if (!= _actor_team_number (Variables|Default|GetAI%20Team%20Number))
    (Class|BPICanbeDamaged|TakeDamage(Message) Actor (Utilities|Struct|MakeS_DamageInfo 2e+01 "NewEnumerator3" "NewEnumerator1") self)))

(event Custom|AI%20Boss%20Attacks:%20Throw%20Weapon
  (params (AI%20Attack%20Target :type Actor%20Object%20Reference))
  ;[0.7999 0.8475 1] AI Boss: Attacks
  (CallFunction|AIAttack AI%20Attack%20Target)
  (bind _notifyname (Animation|Montage|PlayMontage (Variables|Character|GetMesh) "/Game/Animations/Axe/Montage_Axe_Throw.Montage_Axe_Throw")
    (:OnCompleted
      (Rendering|SetVisibility (Variables|/Game/CombatSystem/Improved_AI/AI_Functionality/Actors/BP_Base_Equipabble.BP_Base_Equipabble_C|GetItemStaticMesh (Variables|Default|GetAI%20Weapon)) true false :!label _label)
      (CallFunction|AIEndAttack AI%20Attack%20Target))
    (:OnInterrupted
      (goto _label))
    (:OnNotifyBegin
      (switch name _notifyname
        (:Throw%20Weapon
          (Rendering|SetVisibility (Variables|/Game/CombatSystem/Improved_AI/AI_Functionality/Actors/BP_Base_Equipabble.BP_Base_Equipabble_C|GetItemStaticMesh (Variables|Default|GetAI%20Weapon)) false false)
          (bind _returnvalue (Game|SpawnActorfromClass "/Game/CombatSystem/Improved_AI/Improved_DamageSystem/Projectiles/BP_Projectile_BossWeapon.BP_Projectile_BossWeapon_C" (Math|Transform|MakeTransform (Transformation|GetSocketLocation (Variables|Character|GetMesh) "RightBossWeapon") "0, 0, 0" "1.000000,1.000000,1.000000") "Undefined" "MultiplyWithRoot" 0 4e+03 0.0 AI%20Attack%20Target true self))
          (EventDispatchers|AssignOnProjectileCollision _returnvalue (delegate Custom|On%20Projectile%20Collision_Event)))))))

(event Custom|On%20Projectile%20Collision_Event
  (params (OtherActor :type Actor%20Object%20Reference) (Hit :type Hit%20Result%20Structure))
  ;[0.7999 0.8475 1] AI Boss: Attacks
  (Class|BPICanbeDamaged|TakeDamage(Message) OtherActor (Utilities|Struct|MakeS_DamageInfo 1e+01 "NewEnumerator2" "NewEnumerator1" false true) self))

(event Custom|AI%20Boss%20Attacks:%20Quick%20Attack
  (params (Actor%20Attack%20Target :type Actor%20Object%20Reference))
  ;[0.7999 0.8475 1] AI Boss: Attacks
  (Default|ActorMeleeAttack:ShortRange (Variables|Default|GetBAC_Universal_Attacks) (Utilities|Struct|MakeS_AttackInfo Actor%20Attack%20Target "/Game/Animations/Axe/AM_AI_Boss_QuickAttack.AM_AI_Boss_QuickAttack" (Utilities|Struct|MakeS_DamageInfo 1e+01 "NewEnumerator1" "NewEnumerator3" false true true)) 2e+01))

(event Custom|AI%20Boss%20Attacks:%20Jump%20Attack
  (params (AI%20Attack%20Target :type Actor%20Object%20Reference))
  ;[0.7999 0.8475 1] AI Boss: Attacks
  (Default|ActorMeleeAttack:LongRange (Variables|Default|GetBAC_Universal_Attacks) (Utilities|Struct|MakeS_AttackInfo AI%20Attack%20Target "/Game/Animations/Axe/AM_AI_Boss_JumpAttack.AM_AI_Boss_JumpAttack" (Utilities|Struct|MakeS_DamageInfo 3e+01 "NewEnumerator3" "NewEnumerator4" false false false true)) 2e+01))

(event Custom|AI%20Boss%20Attacks:%20Ground%20Smash
  (params (Actor%20Attack%20Target :type Actor%20Object%20Reference))
  ;[0.7999 0.8475 1] AI Boss: Attacks
  (Default|UniversalAttack:GroundSmash (Variables|Default|GetBAC_Universal_Attacks) (Utilities|Struct|MakeS_AttackInfo Actor%20Attack%20Target "/Game/Animations/Axe/AM_AI_Boss_GroundSmash.AM_AI_Boss_GroundSmash" (Utilities|Struct|MakeS_DamageInfo 5e+01 "NewEnumerator3" "NewEnumerator0" false false false true)) 8e+02))

(event Custom|AI%20Boss%20Attacks:%20Enter%20Floating%20Platform
  (bind _returnvalue (Transformation|GetActorLocation))
  ;[0.7999 0.8475 1] AI Boss: Floating Platform
  (Class|BPICanbeDamaged|IsActorInvinsible(Message) (Variables|Default|GetBAC_DamageSystem) true)
  (bind _outhit (Collision|LineTraceByChannel _returnvalue (* _returnvalue "1.000000,1.000000,-1000.000000") "TraceTypeQuery1" false 0 "None"))
  (bind _returnvalue_2 (Game|SpawnActorfromClass "/Game/CombatSystem/Improved_AI/Props/BP_FloatingPlatform.BP_FloatingPlatform_C" (Math|Transform|MakeTransform (.Location (Collision|BreakHitResult _outhit)) "0, 0, 0" "1.000000,1.000000,1.000000") "Undefined" "MultiplyWithRoot" 0 0))
  (bind _output_get (Variables|Default|SetAI%20Boss%20Floating%20Platform _returnvalue_2))
  (EventDispatchers|AssignOnPlatformFloatTimelineEnd _output_get (delegate Custom|On%20Platform%20Float%20Timeline%20End_Event)))

(event Custom|On%20Platform%20Float%20Timeline%20End_Event
  ;[0.7999 0.8475 1] AI Boss: Floating Platform
  (EventDispatchers|UnbindEventfromOnPlatformFloatTimelineEnd (stale Custom|AI%20Boss%20Attacks:%20Enter%20Floating%20Platform _output_get) (delegate Custom|On%20Platform%20Float%20Timeline%20End_Event))
  (Default|CallOnFloatingPlatformCombatReady))

(event Custom|AI%20Boss%20Attacks:%20Exit%20Floating%20Platform
  ;[0.7999 0.8475 1] AI Boss: Floating Platform
  (bind _ai_boss_floating_platform (Variables|Default|GetAI%20Boss%20Floating%20Platform)
    (:then
      (Default|StopPlatformFloat _ai_boss_floating_platform)
      (EventDispatchers|AssignOnPlatformFloatTimelineEnd _ai_boss_floating_platform (delegate Custom|On%20Platform%20Float%20Timeline%20End_Event_0)))
    (:else
      (Utilities|FlowControl|DelayUntilNextTick)
      (Class|BPICanbeDamaged|IsActorInvinsible(Message) (Variables|Default|GetBAC_DamageSystem) false)
      (Default|CallOnFloatingPlatformCombatDisengage))))

(event EventBeginPlay
  (bind _bac_damagesystem (Variables|Default|GetBAC_DamageSystem))
  (|CallParentFunction)
  ;[0.7999 0.8475 1] AI Boss Health Bar Initialisation
  (UserInterface|SetWidget (Variables|Default|GetAI%20Health%20Bar) 0)
  (bind _returnvalue (UserInterface|CreateWidget "/Game/CombatSystem/Improved_AI/Widgets/WBP_Boss_HP.WBP_Boss_HP_C"))
  (bind _output_get (Variables|Default|SetBoss%20Healthbar%20Widget _returnvalue))
  (Default|UpdateBossHealthPercentage _output_get (Variables|/Game/CombatSystem/Improved_AI/Improved_DamageSystem/BAC_DamageSystem.BAC_DamageSystem_C|GetActor%20Current%20Health _bac_damagesystem) (Variables|/Game/CombatSystem/Improved_AI/Improved_DamageSystem/BAC_DamageSystem.BAC_DamageSystem_C|GetActor%20Max%20Health _bac_damagesystem)))

(event EventAIEquipWeapon
  ;[0.7999 0.8475 1] AI Boss Equip/Unequip Weapon
  (bind _returnvalue (Game|SpawnActorfromClass "/Game/CombatSystem/Improved_AI/AI_Functionality/Actors/BP_Boss_Weapon.BP_Boss_Weapon_C" (Math|Transform|MakeTransform "0, 0, 0" "0, 0, 0" "1.000000,1.000000,1.000000") "Undefined" "MultiplyWithRoot" 0 0))
  (bind _output_get (Variables|Default|SetAI%20Weapon _returnvalue))
  (Default|AttachActor _output_get "RightBossWeapon" (Variables|Character|GetMesh))
  (Variables|Default|SetbIs%20AI%20Weilding%20Weapon true)
  (Utilities|FlowControl|DelayUntilNextTick)
  (Default|CallOnAIUnsheatheWeapon))

(event EventAIUnequipWeapon
  ;[0.7999 0.8475 1] AI Boss Equip/Unequip Weapon
  (Actor|DestroyActor (Variables|Default|GetAI%20Weapon))
  (Variables|Default|SetbIs%20AI%20Weilding%20Weapon false)
  (Utilities|FlowControl|DelayUntilNextTick)
  (Default|CallOnAISheatheWeapon))

(fn ConstructionScript
  (bind _bac_damagesystem (Variables|Default|GetBAC_DamageSystem))
  (|CallParentFunction)
  (bind _output_get (Variables|/Game/CombatSystem/Improved_AI/Improved_DamageSystem/BAC_DamageSystem.BAC_DamageSystem_C|SetActor%20Max%20Health _bac_damagesystem 3e+02))
  (Variables|/Game/CombatSystem/Improved_AI/Improved_DamageSystem/BAC_DamageSystem.BAC_DamageSystem_C|SetActor%20Current%20Health _bac_damagesystem _output_get))

(fn ChangeAIMovementSpeed
  (params (AI%20Movement%20Speed :type E_AI_MovementSpeeds%20Enum :default "NewEnumerator0"))
  (bind _output_get (Variables|/Script/Engine.CharacterMovementComponent|SetMaxWalkSpeed (Variables|Character|GetCharacterMovement) (Utilities|Select :Index AI%20Movement%20Speed :NewEnumerator0 0.0 :NewEnumerator1 1e+02 :NewEnumerator2 2e+02 :NewEnumerator3 3.5e+02)))
  (return _output_get))

(fn TakeDamage
  (params (DamageInfo :type S%20Damage%20Info%20Structure) (DamageInstigator :type Actor%20Object%20Reference))
  (bind _bac_damagesystem (Variables|Default|GetBAC_DamageSystem))
  (bind _bwasdamaged (|CallParentFunction DamageInfo DamageInstigator))
  (Default|UpdateBossHealthPercentage (Variables|Default|GetBoss%20Healthbar%20Widget) (Variables|/Game/CombatSystem/Improved_AI/Improved_DamageSystem/BAC_DamageSystem.BAC_DamageSystem_C|GetActor%20Current%20Health _bac_damagesystem) (Variables|/Game/CombatSystem/Improved_AI/Improved_DamageSystem/BAC_DamageSystem.BAC_DamageSystem_C|GetActor%20Max%20Health _bac_damagesystem))
  (return _bwasdamaged))

(fn GetActorWeapon
  (return (Variables|Default|GetAI%20Weapon)))