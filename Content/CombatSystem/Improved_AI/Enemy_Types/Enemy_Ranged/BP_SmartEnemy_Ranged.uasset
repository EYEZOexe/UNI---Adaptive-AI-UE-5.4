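; Ranged smart enemy that attacks its target with a throw animation and a blockable projectile, built on a parent AI class.
; On BeginPlay it spawns a base weapon, attaches it to the right-hand socket and signals the unsheathe.
; Montage notifies launch the projectile from the weapon toward the target's location, and completion or interruption ends the attack.
; Functions supply attack and defend ranges and map movement states to walk speeds.
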(event EventBeginPlay
  (|CallParentFunction)
  (CallFunction|AIEquipWeapon))

(event EventAIEquipWeapon
  (bind _returnvalue (Game|SpawnActorfromClass "/Game/CombatSystem/Improved_AI/AI_Functionality/Actors/BP_Base_Weapon.BP_Base_Weapon_C" (Math|Transform|MakeTransform "0, 0, 0") "Undefined" "MultiplyWithRoot" 0 0))
  (bind _output_get (Variables|Default|SetAI%20Weapon _returnvalue))
  (Transformation|AttachComponentToComponent _output_get (Variables|Character|GetMesh) "RightWeaponSocket" "SnapToTarget" "SnapToTarget" "SnapToTarget" true)
  (Variables|Default|SetbIs%20AI%20Weilding%20Weapon true)
  (Default|CallOnAIUnsheatheWeapon))

(event EventAIAttack
  (params (AI%20Attack%20Target :type Actor%20Object%20Reference))
  (|CallParentFunction AI%20Attack%20Target)
  (bind _notifyname (Animation|Montage|PlayMontage (Variables|Character|GetMesh) "/Game/AM_AI_Throw_Test.AM_AI_Throw_Test")
    (:OnCompleted
      (CallFunction|AIEndAttack AI%20Attack%20Target :!label _label))
    (:OnInterrupted
      (goto _label))
    (:OnNotifyBegin
      (switch name _notifyname
        (:Throw
          (Default|Regular:Projectile (Variables|Default|GetBAC_Universal_Attacks) (Transformation|GetActorLocation (Variables|Default|GetAI%20Weapon)) (Transformation|GetActorLocation AI%20Attack%20Target) (Utilities|Struct|MakeS_DamageInfo 15.0 "NewEnumerator2" "NewEnumerator0" false true)))))))

(fn ConstructionScript
  (|CallParentFunction))

(fn ChangeAIMovementSpeed
  (params (AI%20Movement%20Speed :type E_AI_MovementSpeeds%20Enum :default "NewEnumerator0"))
  (Variables|/Script/Engine.CharacterMovementComponent|SetMaxWalkSpeed (Variables|Character|GetCharacterMovement) (Utilities|Select :Index AI%20Movement%20Speed :NewEnumerator0 0.0 :NewEnumerator1 1e+02 :NewEnumerator2 3e+02 :NewEnumerator3 5e+02))
  (return 0.0))

(fn GetAIRange
  (return 6e+02 6e+02))