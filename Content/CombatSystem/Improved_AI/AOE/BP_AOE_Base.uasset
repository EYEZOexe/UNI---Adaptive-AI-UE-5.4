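; Base actor for area-of-effect hits in the combat system, reporting every pawn caught within a radius of itself.
; It can auto-start shortly after BeginPlay, or be triggered through StartAOESphere.
; A single sphere overlap, optionally ignoring the instigator and drawing a debug sphere, gathers the pawns.
; Each one is broadcast through the OnAOECollisionWithActor dispatcher, so this base applies no effect itself.
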(event Custom|Start%20AOE%20Sphere
  (CallFunction|SpawnAOESphere))

(event Custom|Spawn%20AOE%20Sphere
  (if (Variables|Default|GetbShouldRunDebug)
    (Rendering|Debug|DrawDebugSphere (Transformation|GetActorLocation) (Variables|Default|GetAOE%20Radius) 12 "(R=1.000000,G=0.000000,B=0.802695,A=1.000000)" 1.0 1.0))
  (bind _outactors (Collision|SphereOverlapActors (Transformation|GetActorLocation) (Variables|Default|GetAOE%20Radius) (Utilities|Array|MakeArray "ObjectTypeQuery3") 0 (Utilities|Array|MakeArray (select (Variables|Default|GetbShouldIgnoreInstigator) (Variables|Actor|GetInstigator) 0))))
  (for _array_element _outactors
    (Default|CallOnAOECollisionwithActor _array_element)))

(event EventBeginPlay
  (if (Variables|Default|GetbShouldRunAtBeginPlay)
    (Utilities|FlowControl|Delay 0.1)
    (CallFunction|StartAOESphere)))

(fn ConstructionScript)