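; Base Blueprint for AOE blast actors in the combat damage system, adding one-shot particle and sound feedback to the parent AOE logic.
; When triggered, it runs the parent's AOE trigger, then spawns the blast emitter and plays the blast sound at the actor's location.
; The actor destroys itself when the particle system finishes, or after a short fallback delay if no valid effect spawned.
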(event Custom|OnSystemFinished_Event
  (params (PSystem :type Particle%20System%20Component%20Object%20Reference))
  (Actor|DestroyActor))

(event Custom|Play%20AOE%20Blast%20Sound
  (bind _blastsound (Variables|Default|GetBlastSound)
    (:then
      (Audio|PlaySoundatLocation _blastsound (Transformation|GetActorLocation) "0, 0, 0" 1.0 1.0 0.0 0 0 0 0))
    (:else)))

(event Custom|Spawn%20AOE%20Blast%20Effect
  (bind _blasteffect (Variables|Default|GetBlastEffect)
    (:then
      (bind _returnvalue (Effects|SpawnEmitteratLocation _blasteffect (Transformation|GetActorLocation)))
      (Variables|Default|SetSpawnedEffect _returnvalue))
    (:else)))

(event Custom|Start%20AOE%20Sphere_1
  (|CallParentFunction)
  (CallFunction|SpawnAOEBlastEffect)
  (CallFunction|PlayAOEBlastSound)
  (bind _spawnedeffect (Variables|Default|GetSpawnedEffect)
    (:then
      (EventDispatchers|AssignOnSystemFinished _spawnedeffect (delegate Custom|OnSystemFinished_Event)))
    (:else
      (Utilities|FlowControl|Delay 3.0)
      (Actor|DestroyActor))))

(event EventBeginPlay
  (|CallParentFunction) ; This node is disabled and will not be called.\nDrag off pins to build functionality.
)

(fn ConstructionScript
  (|CallParentFunction))