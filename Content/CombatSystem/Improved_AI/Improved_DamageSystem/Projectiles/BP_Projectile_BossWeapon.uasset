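; Boss weapon projectile Blueprint that spins its axe as soon as it begins play, after running the parent's BeginPlay.
; A timeline drives the world yaw of the axe rotation point while keeping its current pitch and roll.
; The spin event calls itself when the timeline finishes, so the rotation loops indefinitely without using Tick.
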(event Custom|Spin%20Boss%20Weapon
  (bind _axe_rotation_point (Variables|Default|GetAxe%20Rotation%20Point))
  (bind _returnvalue (Transformation|GetWorldRotation _axe_rotation_point))
  (bind _rotation__z_axis (Timeline|Rotation%20of%20Axe%20Timeline PlayFromStart)
    (:Update
      (Transformation|SetWorldRotation (Variables|Default|GetAxe%20Rotation%20Point) (Math|Rotator|MakeRotator (.roll _returnvalue) (.pitch _returnvalue) _rotation__z_axis) false false))
    (:Finished
      (CallFunction|SpinBossWeapon))))

(event EventBeginPlay
  (|CallParentFunction)
  (CallFunction|SpinBossWeapon))

(event Collision|EventActorBeginOverlap
  (params (OtherActor :type Actor%20Object%20Reference)))

(event EventTick
  (params (DeltaSeconds :type Float%20%28single-precision%29)))

(fn ConstructionScript
  (|CallParentFunction))