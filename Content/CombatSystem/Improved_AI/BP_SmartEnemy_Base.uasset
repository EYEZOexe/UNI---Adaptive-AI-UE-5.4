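; Base enemy character that connects the BAC damage system component to AIC_SmartEnemy_Base states, driving hit reactions, retargeting and ragdoll death.
; Attacks take tokens from the target, tracked per target and returned when the attack ends or the enemy dies.
; Blockable hits roll a chance for a timed block.
; Navlink jumps use a projectile-arc launch, while teleport evade is a hidden, high-speed flying AIMoveTo with pawn collision ignored.
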(event OnActorBlockedEvent(BAC_DamageSystem)
  (params (CanBeParried :type Boolean) (Damage%20Instigator :type Actor%20Object%20Reference))
  ;[0.776 0.03342 0] AI Blocking States
  (Utilities|Time|ClearandInvalidateTimerbyHandle (Variables|Default|GetAI%20Block%20Timer))
  (Animation|Montage|PlayMontage (Variables|Character|GetMesh) (Variables|AIInitialisation|Montages|GetAI%20Block%20Reaction%20Montage)
    (:OnCompleted
      _)
    (:OnInterrupted
      _))
  (CallFunction|ExitAIBlockingState))

(event Custom|AI%20Magic:%20Enter%20Teleport%20Evade
  (params (Teleport%20Location :type Vector) (AI%20Attack%20Target :type Actor%20Object%20Reference))
  (bind _charactermovement (Variables|Character|GetCharacterMovement))
  (bind _mesh (Variables|Character|GetMesh))
  ;[0.7999 0.8475 1] AI Magic: Teleport
  (if (not (Variables|Default|GetbIs%20AI%20Actor%20Teleporting))
    (Variables|Default|SetbIs%20AI%20Actor%20Teleporting true)
    (Pawn|Components|CharacterMovement|SetMovementMode _charactermovement "MOVE_Flying" 0)
    (Variables|/Script/Engine.CharacterMovementComponent|SetMaxFlySpeed _charactermovement 5e+03)
    (Variables|/Script/Engine.CharacterMovementComponent|SetMaxAcceleration _charactermovement 99999.0)
    (Rendering|SetVisibility _mesh false true)
    (Collision|SetCollisionResponsetoChannel (Variables|Collision|GetCapsuleComponent) "ECC_Pawn" "ECR_Ignore")
    (bind _returnvalue (Effects|SpawnEmitterAttached (Variables|Default|GetAI%20Teleport%20Effect%20Particle) _mesh (Variables|AIInitialisation|GetAI%20Teleport%20Effect%20Socket%20Name)))
    (Variables|AIInitialisation|SetAI%20Teleport%20Particle%20Effect _returnvalue)
    (bind _returnvalue_2 (Effects|SpawnEmitterAttached (Variables|Default|GetAI%20Teleport%20Trail%20Particle) _mesh (Variables|AIInitialisation|GetAI%20Teleport%20Trail%20Effect%20Socket%20Name)))
    (Variables|AIInitialisation|SetAI%20Teleport%20Trail%20Effect _returnvalue_2)
    (Animation|StopAnimMontage 0)
    (AI|AIMoveTo self Teleport%20Location AI%20Attack%20Target (Variables|AIInitialisation|GetAI%20Teleport%20Acceptance%20Radius) false
      (:OnSuccess
        _)
      (:OnFail
        _))
    (CallFunction|AIMagic:ExitTeleportEvade)
    (else
      (Utilities|FlowControl|DelayUntilNextTick)
      (Default|CallOnAITeleportExit))))

(event Custom|AI%20Magic:%20Exit%20Teleport%20Evade
  (bind _charactermovement (Variables|Character|GetCharacterMovement))
  ;[0.7999 0.8475 1] AI Magic: Teleport
  (Components|Movement|StopMovementImmediately _charactermovement)
  (Pawn|Components|CharacterMovement|SetMovementMode _charactermovement "MOVE_Walking" 0)
  (Variables|/Script/Engine.CharacterMovementComponent|SetMaxAcceleration _charactermovement 1.5e+03)
  (Rendering|SetVisibility (Variables|Character|GetMesh) true true)
  (Collision|SetCollisionResponsetoChannel (Variables|Collision|GetCapsuleComponent) "ECC_Pawn" "ECR_Block")
  (Default|CallOnAITeleportExit)
  (Utilities|FlowControl|Delay 0.5)
  (Variables|Default|SetbIs%20AI%20Actor%20Teleporting false)
  (Utilities|FlowControl|Sequence
    (:then_0
      (bind _ai_teleport_particle_effect (Variables|AIInitialisation|GetAI%20Teleport%20Particle%20Effect)
        (:then
          (Components|DestroyComponent _ai_teleport_particle_effect))
        (:else)))
    (:then_1
      (bind _ai_teleport_trail_effect (Variables|AIInitialisation|GetAI%20Teleport%20Trail%20Effect)
        (:then
          (Components|DestroyComponent _ai_teleport_trail_effect))
        (:else)))))

(event Custom|On%20AI%20Death
  (bind _mesh (Variables|Character|GetMesh))
  (bind _aic_smart_enemy_base (Variables|Default|GetAIC%20Smart%20Enemy%20Base))
  ;[0.7999 0.8475 1] AI Death Event
  (Animation|StopAnimMontage 0)
  (Physics|SetSimulatePhysics _mesh true)
  (Collision|SetCollisionEnabled _mesh "QueryAndPhysics")
  (AI|Logic|StopLogic (Variables|/Script/AIModule.AIController|GetBrainComponent _aic_smart_enemy_base) "Dead")
  (Default|SetAIState:Dead _aic_smart_enemy_base)
  (Rendering|SetVisibility (Variables|Default|GetAI%20Health%20Bar) false true)
  (bind _keys (Utilities|Map|Keys (Variables|Default|GetAI%20Stored%20Attack%20Tokens)))
  (for _array_element _keys
    (Class|BPICanbeDamaged|GiveActorAttackToken(Message) _array_element (.Value (Utilities|Map|Find (Variables|Default|GetAI%20Stored%20Attack%20Tokens) _array_element)))))

(event Custom|On%20AI%20Damage%20Response
  (params (DamageResponse :type E_DamageResponse%20Enum :default "NewEnumerator0") (Damage%20Instigator :type Actor%20Object%20Reference))
  (bind _ai_hit_reaction_montage (Variables|AIInitialisation|Montages|GetAI%20Hit%20Reaction%20Montage))
  (bind _ai_stagger_reaction_montage (Variables|AIInitialisation|Montages|GetAI%20Stagger%20Reaction%20Montage))
  ;[1 0 0.007827] AI Hit Response
  (Components|Movement|StopMovementImmediately (Variables|Character|GetCharacterMovement))
  (Default|SetAIState:Stunned (Variables|Default|GetAIC%20Smart%20Enemy%20Base))
  (Animation|Montage|PlayMontage (Variables|Character|GetMesh) (Utilities|Select :Index DamageResponse :NewEnumerator0 _ai_hit_reaction_montage :NewEnumerator1 _ai_hit_reaction_montage :NewEnumerator2 (select (Utilities|IsValid _ai_stagger_reaction_montage) _ai_stagger_reaction_montage _ai_hit_reaction_montage) :NewEnumerator3 _ai_hit_reaction_montage :NewEnumerator4 _ai_hit_reaction_montage)
    (:OnCompleted
      _)
    (:OnInterrupted
      _))
  (bind _actor_team_number (Class|BPICanbeDamaged|GetActorTeamNumber(Message) Damage%20Instigator))
  (Default|SetAIState:Attacking (Variables|Default|GetAIC%20Smart%20Enemy%20Base) (select (!= _actor_team_number (Variables|AIInitialisation|GetAI%20Team%20Number)) Damage%20Instigator 0) true))

(event Custom|Enter%20AI%20Blocking%20State
  ;[0.776 0.03342 0] AI Blocking States
  (Utilities|Time|ClearandInvalidateTimerbyHandle (Variables|Default|GetAI%20Block%20Timer))
  (Variables|/Game/CombatSystem/Improved_AI/Improved_DamageSystem/BAC_DamageSystem.BAC_DamageSystem_C|SetbIsActorBlocking (Variables|Default|GetBAC_DamageSystem) true)
  (Components|Movement|StopMovementImmediately (Variables|Character|GetCharacterMovement))
  (bind _returnvalue (Utilities|Time|SetTimerbyEvent (EventDispatchers|CreateEvent :!event Custom|Exit%20AI%20Blocking%20State) 2.0))
  (Variables|Default|SetAI%20Block%20Timer _returnvalue))

(event Custom|Exit%20AI%20Blocking%20State
  ;[0.776 0.03342 0] AI Blocking States
  (Variables|/Game/CombatSystem/Improved_AI/Improved_DamageSystem/BAC_DamageSystem.BAC_DamageSystem_C|SetbIsActorBlocking (Variables|Default|GetBAC_DamageSystem) false)
  (Default|CallOnAIExitBlockingState))

(event EventIsAttackInterruptable
  (params (bIsAttackInterruptable :type Boolean))
  ;[1 0 0] AI Damage System Booleans
  (Variables|/Game/CombatSystem/Improved_AI/Improved_DamageSystem/BAC_DamageSystem.BAC_DamageSystem_C|SetbIsAttackInterruptable (Variables|Default|GetBAC_DamageSystem) bIsAttackInterruptable))

(event EventAIJumptoNavlinkProxy
  (params (Jump%20Destination :type Vector :default "0, 0, 0"))
  (bind (_x _y _z) (Math|Vector|BreakVector Jump%20Destination))
  ;[0.7999 0.8475 1] AI Jump To Navlinks
  (bind _outlaunchvelocity (Game|SuggestProjectileVelocityCustomArc (Transformation|GetActorLocation) (Math|Vector|MakeVector _x _y (+ _z 2.5e+02)) 0.0 0.5))
  (Character|LaunchCharacter _outlaunchvelocity true true))

(event EventGiveActorAttackToken
  (params (Amount%20To%20Give%20Back%20To%20Actor :type Integer))
  ;[0.7999 0.8475 1] Token System Exchange
  (Default|GiveActorAttackToken (Variables|Default|GetBAC_DamageSystem) Amount%20To%20Give%20Back%20To%20Actor))

(event EventBeginPlay
  ;[0.7999 0.8475 1] AI Begin Play
  (bind _asaic_smart_enemy_base (Utilities|Casting|CastToAIC_SmartEnemy_Base (AI|GetAIController self)))
  (Variables|Default|SetAIC%20Smart%20Enemy%20Base _asaic_smart_enemy_base)
  (EventDispatchers|BindEventtoOnActorDeathEvent (Variables|Default|GetBAC_DamageSystem) (EventDispatchers|CreateEvent :!event Custom|On%20AI%20Death))
  (EventDispatchers|BindEventtoOnActorDamageResponse (Variables|Default|GetBAC_DamageSystem) (EventDispatchers|CreateEvent :!event Custom|On%20AI%20Damage%20Response)))

(event EventAIStoredTokenAmount
  (params (AI%20Attack%20Target :type Actor%20Object%20Reference) (Amount%20of%20Tokens%20Taken :type Integer))
  (bind _ai_stored_attack_tokens (Variables|Default|GetAI%20Stored%20Attack%20Tokens))
  (bind (_value _returnvalue) (Utilities|Map|Find _ai_stored_attack_tokens AI%20Attack%20Target))
  ;[0.7999 0.8475 1] Token System Exchange
  (Utilities|Map|Add (Variables|Default|GetAI%20Stored%20Attack%20Tokens) AI%20Attack%20Target (Math|Integer|SelectInt (+ Amount%20of%20Tokens%20Taken _value) Amount%20of%20Tokens%20Taken _returnvalue)))

(event EventAIEndAttack
  (params (AI%20Attack%20Target :type Actor%20Object%20Reference))
  (bind _ai_spent_attack_tokens_on_current_attack (Variables|Default|GetAI%20Spent%20Attack%20Tokens%20On%20Current%20Attack))
  ;[0.7999 0.8475 1] Token System Exchange
  (Class|BPICanbeDamaged|GiveActorAttackToken(Message) AI%20Attack%20Target _ai_spent_attack_tokens_on_current_attack)
  (CallFunction|AIStoredTokenAmount AI%20Attack%20Target (* _ai_spent_attack_tokens_on_current_attack -1))
  (Variables|Default|SetbIs%20AI%20Attacking false)
  (Default|CallOnAIAttackEnd))

(event EventAIAttack
  (params (AI%20Attack%20Target :type Actor%20Object%20Reference))
  ;[1 0 0] AI Damage System Booleans
  (Variables|Default|SetbIs%20AI%20Attacking true))

(event EventIsActorInvinsible
  (params (bIsActorInvinsible :type Boolean))
  ;[1 0 0] AI Damage System Booleans
  (Variables|/Game/CombatSystem/Improved_AI/Improved_DamageSystem/BAC_DamageSystem.BAC_DamageSystem_C|SetbDoesActorHaveInvisibilityFrames (Variables|Default|GetBAC_DamageSystem) bIsActorInvinsible))

(fn ConstructionScript
  (bind _bac_damagesystem (Variables|Default|GetBAC_DamageSystem))
  (Variables|/Game/CombatSystem/Improved_AI/Improved_DamageSystem/BAC_DamageSystem.BAC_DamageSystem_C|SetActor%20Max%20Health _bac_damagesystem 1e+02)
  (Variables|/Game/CombatSystem/Improved_AI/Improved_DamageSystem/BAC_DamageSystem.BAC_DamageSystem_C|SetActor%20Current%20Health _bac_damagesystem 1e+02))

(fn AIPercentileBlock
  (if (<= (Math|Random|RandomFloat) (Variables|AIInitialisation|GetAI%20Percent%20Chance%20To%20Block))
    (CallFunction|EnterAIBlockingState)))

(fn AIStartAttack
  (params (AI%20Attack%20Target :type Actor%20Object%20Reference) (Actor%20Token%20Amount%20Required :type Integer))
  (bind _bwastakingactortokensuccessful (Class|BPICanbeDamaged|TakeActorAttackToken(Message) AI%20Attack%20Target Actor%20Token%20Amount%20Required))
  (if _bwastakingactortokensuccessful
    (CallFunction|AIStoredTokenAmount AI%20Attack%20Target Actor%20Token%20Amount%20Required)
    (Variables|Default|SetAI%20Spent%20Attack%20Tokens%20On%20Current%20Attack Actor%20Token%20Amount%20Required)
    (return true)
    (else
      (return false))))

(fn BIsActorAttacking
  (return (Variables|Default|GetbIs%20AI%20Attacking)))

(fn BIsActorDead
  (return (Variables|/Game/CombatSystem/Improved_AI/Improved_DamageSystem/BAC_DamageSystem.BAC_DamageSystem_C|GetbIsActorDead (Variables|Default|GetBAC_DamageSystem))))

(fn ChangeAIMovementSpeed
  (params (AI%20Movement%20Speed :type E_AI_MovementSpeeds%20Enum :default "NewEnumerator0"))
  (bind _output_get (Variables|/Script/Engine.CharacterMovementComponent|SetMaxWalkSpeed (Variables|Character|GetCharacterMovement) (Utilities|Select :Index AI%20Movement%20Speed :NewEnumerator0 0.0 :NewEnumerator1 1e+02 :NewEnumerator2 3e+02 :NewEnumerator3 5e+02)))
  (return _output_get))

(fn GetActorCurrentHealth
  (return (Variables|/Game/CombatSystem/Improved_AI/Improved_DamageSystem/BAC_DamageSystem.BAC_DamageSystem_C|GetActor%20Current%20Health (Variables|Default|GetBAC_DamageSystem))))

(fn GetActorMaxHealth
  (return (Variables|/Game/CombatSystem/Improved_AI/Improved_DamageSystem/BAC_DamageSystem.BAC_DamageSystem_C|GetActor%20Max%20Health (Variables|Default|GetBAC_DamageSystem))))

(fn GetActorTeamNumber
  (return (Variables|AIInitialisation|GetAI%20Team%20Number)))

(fn GetActorWeapon
  (return (Variables|Default|GetAI%20Weapon)))

(fn GetAIPatrolRoute
  (return (Variables|AIInitialisation|GetAI%20Patrol%20Route)))

(fn GetAIRange
  (return 1.5e+02 3.5e+02))

(fn HealSelf
  (params (HealAmount :type Float%20%28double-precision%29))
  (bind _newhealth (Default|HealSelf (Variables|Default|GetBAC_DamageSystem) HealAmount))
  (return _newhealth))

(fn TakeActorAttackToken
  (params (Amount%20of%20Actor%20Tokens%20To%20Take :type Integer))
  (bind _bwastakingactortokensuccessful (Default|TakeActorAttackToken (Variables|Default|GetBAC_DamageSystem) Amount%20of%20Actor%20Tokens%20To%20Take))
  (return _bwastakingactortokensuccessful))

(fn TakeDamage
  (params (DamageInfo :type S%20Damage%20Info%20Structure) (DamageInstigator :type Actor%20Object%20Reference))
  (if (Utilities|Struct|BreakS_DamageInfo DamageInfo)
    (CallFunction|AIPercentileBlock))
  (bind _wasdamaged (Default|TakeDamage (Variables|Default|GetBAC_DamageSystem) DamageInfo DamageInstigator))
  (return _wasdamaged))